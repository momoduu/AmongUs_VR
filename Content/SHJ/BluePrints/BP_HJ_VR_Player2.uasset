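; VR player Blueprint with Among Us-style sound cues and a screen fade on entering teleport actors.
; Right trigger, left thumbstick press, Y and B play mission-complete, jump, kill and body-found sounds; B also briefly shows CallVote.
; Capsule overlaps cast against six teleport actor classes to call MoveComp.TeleportFade, though the BP_MainMapgoto branch's IsValid has no input.
; The Enhanced Input mapping-context setup is unconnected and never runs.
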(event OnComponentBeginOverlap(CapsuleComponent)
  (params (OverlappedComponent :type Primitive%20Component%20Object%20Reference) (OtherActor :type Actor%20Object%20Reference) (OtherComp :type Primitive%20Component%20Object%20Reference) (OtherBodyIndex :type Integer) (bFromSweep :type Boolean) (SweepResult :type Hit%20Result%20Structure%20%28by%20ref%29))
  ;[1 1 1] 화면 fade in
  (Utilities|FlowControl|Sequence
    (:then_0
      (bind _asbp_goto_aisle (Utilities|Casting|CastToBP_gotoAisle OtherActor))
      (Utilities|IsValid _asbp_goto_aisle
        (:Is%20Valid
          (Class|PlayerMoveComponent|TeleportFade (Variables|Default|GetmoveComp)))))
    (:then_1
      (bind _asbp_aisle_teleport (Utilities|Casting|CastToBP_AisleTeleport OtherActor))
      (Utilities|IsValid _asbp_aisle_teleport
        (:Is%20Valid
          (Class|PlayerMoveComponent|TeleportFade (Variables|Default|GetmoveComp)))))
    (:then_2
      (bind _asbp_goto_mini_game_2 (Utilities|Casting|CastToBP_gotoMiniGame2 OtherActor))
      (Utilities|IsValid _asbp_goto_mini_game_2
        (:Is%20Valid
          (Class|PlayerMoveComponent|TeleportFade (Variables|Default|GetmoveComp)))))
    (:then_3
      (bind _asbp_room_teleport (Utilities|Casting|CastToBP_RoomTeleport OtherActor))
      (Utilities|IsValid _asbp_room_teleport
        (:Is%20Valid
          (Class|PlayerMoveComponent|TeleportFade (Variables|Default|GetmoveComp)))))
    (:then_4
      (bind _asbp_main_map_teleport (Utilities|Casting|CastToBP_MainMapTeleport OtherActor))
      (Utilities|IsValid _asbp_main_map_teleport
        (:Is%20Valid
          (Class|PlayerMoveComponent|TeleportFade (Variables|Default|GetmoveComp)))))
    (:then_5
      (Utilities|Casting|CastToBP_MainMapgoto OtherActor)
      (Utilities|IsValid 0
        (:Is%20Valid
          (Class|PlayerMoveComponent|TeleportFade (Variables|Default|GetmoveComp)))))))

(event Input|EnhancedActionEvents|EnhancedInputActionIA_Y_Press
  (params (ActionValue :type Boolean) (ElapsedSeconds :type Float%20%28double-precision%29) (TriggeredSeconds :type Float%20%28double-precision%29) (InputAction :type Input%20Action%20Object%20Reference :default "/Game/MyInput/IA_Y_Press.IA_Y_Press"))
  (:Started
    (Audio|PlaySound2D "/Game/SHJ/Sound/sound_Wav/임포스터_킬__online-audio-converter_com_.임포스터_킬__online-audio-converter_com_" 1.0 1.0 0.0 0 0)))

(event Input|EnhancedActionEvents|EnhancedInputActionIA_B_Press
  (params (ActionValue :type Boolean) (ElapsedSeconds :type Float%20%28double-precision%29) (TriggeredSeconds :type Float%20%28double-precision%29) (InputAction :type Input%20Action%20Object%20Reference :default "/Game/MyInput/IA_B_Press.IA_B_Press"))
  (bind _callvote (Variables|Default|GetCallVote))
  (:Started
    (Audio|PlaySound2D "/Game/SHJ/Sound/sound_Wav/시체_발견.시체_발견" 1.0 1.0 0.0 0 0)
    (Rendering|SetVisibility _callvote true false)
    (Utilities|FlowControl|Delay 2.0)
    (Rendering|SetVisibility _callvote false false)))

(event Input|EnhancedActionEvents|EnhancedInputActionIA_ThumbStickPress_left
  (params (ActionValue :type Boolean) (ElapsedSeconds :type Float%20%28double-precision%29) (TriggeredSeconds :type Float%20%28double-precision%29) (InputAction :type Input%20Action%20Object%20Reference :default "/Game/MyInput/IA_ThumbStickPress_left.IA_ThumbStickPress_left"))
  (:Started
    (Audio|PlaySound2D "/Game/SHJ/Sound/sound_Wav/jump.jump" 1.0 1.0 0.0 0 0)))

(event Input|EnhancedActionEvents|EnhancedInputActionIA_Trigger_Right
  (params (ActionValue :type Boolean) (ElapsedSeconds :type Float%20%28double-precision%29) (TriggeredSeconds :type Float%20%28double-precision%29) (InputAction :type Input%20Action%20Object%20Reference :default "/Game/MyInput/IA_Trigger_Right.IA_Trigger_Right"))
  (:Started
    (Audio|PlaySound2D "/Game/SHJ/Sound/sound_Wav/임무_완료.임무_완료" 1.0 1.0 0.0 0 0)))

(event EventBeginPlay)

(event Collision|EventActorBeginOverlap
  (params (OtherActor :type Actor%20Object%20Reference))
  ;[1 1 1] 화면 fade in
)

(event EventTick
  (params (DeltaSeconds :type Float%20%28single-precision%29))
  ;[1 1 1] 화면 fade in
)

(fn ConstructionScript)