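; Room exit trigger that sends the player to the Aisle level.
; Overlapping its box plays a player-exit sound, then opens the level by name after a short delay, without checking which actor overlapped.
; On BeginPlay it briefly shows a look-around widget and caches a BP_AisleTeleport reference that is not used here.
; A call to show GotoA2 is left unconnected.
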(event OnComponentBeginOverlap(Box)
  (params (OverlappedComponent :type Primitive%20Component%20Object%20Reference) (OtherActor :type Actor%20Object%20Reference) (OtherComp :type Primitive%20Component%20Object%20Reference) (OtherBodyIndex :type Integer) (bFromSweep :type Boolean) (SweepResult :type Hit%20Result%20Structure%20%28by%20ref%29))
  (Audio|PlaySound2D "/Game/SHJ/Sound/sound_Wav/플레이어_퇴장.플레이어_퇴장" 1.0 1.0 0.0 0 0)
  (Utilities|FlowControl|Delay 2.0)
  (Game|OpenLevel(byName) "Aisle"))

(event OnComponentEndOverlap(Box)
  (params (OverlappedComponent :type Primitive%20Component%20Object%20Reference) (OtherActor :type Actor%20Object%20Reference) (OtherComp :type Primitive%20Component%20Object%20Reference) (OtherBodyIndex :type Integer)))

(event EventBeginPlay
  (bind _lookaroundwidget (Variables|Default|GetlookAroundWidget))
  (bind _returnvalue (Actor|GetActorOfClass "/Game/SHJ/BluePrints/BP_AisleTeleport.BP_AisleTeleport_C"))
  (Variables|Default|SetaisleTeleport _returnvalue)
  (Rendering|SetVisibility _lookaroundwidget true false)
  (Utilities|FlowControl|Delay 5.0)
  (Rendering|SetVisibility _lookaroundwidget false false))

(event Collision|EventActorBeginOverlap
  (params (OtherActor :type Actor%20Object%20Reference)))

(event EventTick
  (params (DeltaSeconds :type Float%20%28single-precision%29)))

(fn ConstructionScript)