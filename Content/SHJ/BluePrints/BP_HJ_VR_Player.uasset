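; BP_HJ_VR_Player is a VR player Blueprint that fades the screen when the player enters a map teleport or goto trigger.
; Capsule begin-overlap runs a sequence of casts against six trigger classes, calling TeleportFade on MoveComp for valid matches.
; The BP_MainMapgoto branch leaves its IsValid input unconnected, so that check cannot pass.
; An Enhanced Input mapping-context node is present but never executes.
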(event OnComponentBeginOverlap(CapsuleComponent)
  (params (OverlappedComponent :type Primitive%20Component%20Object%20Reference) (OtherActor :type Actor%20Object%20Reference) (OtherComp :type Primitive%20Component%20Object%20Reference) (OtherBodyIndex :type Integer) (bFromSweep :type Boolean) (SweepResult :type Hit%20Result%20Structure%20%28by%20ref%29))
  ;[1 1 1] 화면 fade in
  (Utilities|FlowControl|Sequence
    (:then_0
      (bind _asbp_goto_aisle (Utilities|Casting|CastToBP_gotoAisle OtherActor))
      (Utilities|IsValid _asbp_goto_aisle
        (:Is%20Valid
          (Class|PlayerMoveComponent|TeleportFade (Variables|Default|GetmoveComp)))))
    (:then_1
      (bind _asbp_aisle_teleport (Utilities|Casting|CastToBP_AisleTeleport OtherActor))
      (Utilities|IsValid _asbp_aisle_teleport
        (:Is%20Valid
          (Class|PlayerMoveComponent|TeleportFade (Variables|Default|GetmoveComp)))))
    (:then_2
      (bind _asbp_goto_mini_game_2 (Utilities|Casting|CastToBP_gotoMiniGame2 OtherActor))
      (Utilities|IsValid _asbp_goto_mini_game_2
        (:Is%20Valid
          (Class|PlayerMoveComponent|TeleportFade (Variables|Default|GetmoveComp)))))
    (:then_3
      (bind _asbp_room_teleport (Utilities|Casting|CastToBP_RoomTeleport OtherActor))
      (Utilities|IsValid _asbp_room_teleport
        (:Is%20Valid
          (Class|PlayerMoveComponent|TeleportFade (Variables|Default|GetmoveComp)))))
    (:then_4
      (bind _asbp_main_map_teleport (Utilities|Casting|CastToBP_MainMapTeleport OtherActor))
      (Utilities|IsValid _asbp_main_map_teleport
        (:Is%20Valid
          (Class|PlayerMoveComponent|TeleportFade (Variables|Default|GetmoveComp)))))
    (:then_5
      (Utilities|Casting|CastToBP_MainMapgoto OtherActor)
      (Utilities|IsValid 0
        (:Is%20Valid
          (Class|PlayerMoveComponent|TeleportFade (Variables|Default|GetmoveComp)))))))

(event EventBeginPlay)

(event Collision|EventActorBeginOverlap
  (params (OtherActor :type Actor%20Object%20Reference)))

(event EventTick
  (params (DeltaSeconds :type Float%20%28single-precision%29)))

(fn ConstructionScript)