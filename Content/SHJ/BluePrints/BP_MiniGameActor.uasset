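; Mini-game actor that shows a password-entry prompt when something enters its collision box.
; On BeginPlay it casts MiniGameWidget's widget to BP_HJ_MiniGameWidget and hands it a reference to WrongWidget.
; Box overlap shows TxtWidget and calls EnableInput through player controller 0, and end overlap reverses both.
; The overlap events do not filter the overlapping actor, and the puzzle logic is outside this Blueprint.
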(event OnComponentBeginOverlap(Box)
  (params (OverlappedComponent :type Primitive%20Component%20Object%20Reference) (OtherActor :type Actor%20Object%20Reference) (OtherComp :type Primitive%20Component%20Object%20Reference) (OtherBodyIndex :type Integer) (bFromSweep :type Boolean) (SweepResult :type Hit%20Result%20Structure%20%28by%20ref%29))
  ;[1 1 1] Collision 닿았을 때 암호 입력 알림
  (Rendering|SetVisibility (Variables|Default|Gettxt_Widget) true false)
  (Input|EnableInput (Game|GetPlayerController 0) 0))

(event OnComponentEndOverlap(Box)
  (params (OverlappedComponent :type Primitive%20Component%20Object%20Reference) (OtherActor :type Actor%20Object%20Reference) (OtherComp :type Primitive%20Component%20Object%20Reference) (OtherBodyIndex :type Integer))
  ;[1 1 1] Collision 닿았을 때 암호 입력 알림
  (Rendering|SetVisibility (Variables|Default|Gettxt_Widget) false false)
  (Input|DisableInput (Game|GetPlayerController 0) 0))

(event EventBeginPlay
  (bind _asbp_hj_mini_game_widget (Utilities|Casting|CastToBP_HJ_MiniGameWidget (UserInterface|GetWidget (Variables|Default|GetMiniGameWidget))))
  (Variables|/Game/SHJ/UI/BP_HJ_MiniGameWidget.BP_HJ_MiniGameWidget_C|SetwrongWidget _asbp_hj_mini_game_widget (Variables|Default|GetwrongWidget)))

(event Collision|EventActorBeginOverlap
  (params (OtherActor :type Actor%20Object%20Reference)))

(event EventTick
  (params (DeltaSeconds :type Float%20%28single-precision%29)))

(fn ConstructionScript)